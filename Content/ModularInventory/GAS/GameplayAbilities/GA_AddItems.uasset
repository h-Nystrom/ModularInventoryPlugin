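; GA_AddItems is an event-triggered Gameplay Ability that picks up an item into the player's inventory.
; After committing, it checks that the event's Instigator implements I_Item and passes its item data to TryAddItem on the ThirdPersonCharacter avatar's Inventory component.
; Success destroys the item actor, while failure only prints the rest amount.
; Debug prints report each failed check, and every path except a missing inventory ends the ability.
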(event `self.K2_ActivateAbilityFromEvent`
  (params (EventData :type "GameplayEventData Structure (by ref)"))
  (bind (_eventtag _instigator) (break `GameplayEventData` (`self.CurrentEventData`)))
  (bind _returnvalue (`self.K2_CommitAbility`))
  (if _returnvalue
    (if (`KismetSystemLibrary.DoesImplementInterface` (`.Instigator` (break `GameplayEventData` EventData)) "/ModularInventory/Interfaces/I_Item.I_Item_C")
      (bind _asthird_person_character (cast `/Game/Players/ThirdPersonCharacter` (`self.GetAvatarActorFromActorInfo`))
        (:`then`
          (bind _returnvalue_2 (`Actor.GetComponentByClass` _asthird_person_character "/Script/ModularInventory.Inventory"))
          (`/Engine/EditorBlueprintResources/StandardMacros.IsValid` _returnvalue_2
            (:`Is Valid`
              (bind _itemdata (message `/ModularInventory/Interfaces/I_Item.GetItemData` _instigator))
              (bind (_restamount _returnvalue_3) (`Inventory.TryAddItem` _returnvalue_2 _itemdata))
              (if _returnvalue_3
                (`KismetSystemLibrary.PrintString` "Done")
                (`Actor.K2_DestroyActor` _instigator)
                (`self.K2_EndAbility`)
                (else
                  (`KismetSystemLibrary.PrintString` (`KismetStringLibrary.Concat_StrStr` "Rest amount: " (`KismetStringLibrary.Conv_IntToString` _restamount)) true true (struct :`R` 1.0 :`G` 0.949602 :`A` 1.0) 10.0)
                  (`self.K2_EndAbility`))))
            (:`Is Not Valid`
              (`KismetSystemLibrary.PrintString` "InventoryDoesn'tExist"))))
        (:`CastFailed`
          (`KismetSystemLibrary.PrintString` "CastingToPlayerError" true true (struct :`R` 1.0 :`G` 0.041752 :`A` 1.0) 5.0)
          (`self.K2_EndAbility` :!label _label)))
      (else
        (`KismetSystemLibrary.PrintString` "NotAnItem")
        (goto _label)))
    (else
      (`KismetSystemLibrary.PrintString` "Can'tBranch")
      (`self.K2_EndAbility`))))